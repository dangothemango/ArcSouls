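; ExtraBear is a pickup actor that grants the player an extra bear, described in its graph as a spirit charge.
; From BeginPlay, its IconImage bobs endlessly through chained, eased MoveComponentTo calls that loop back on themselves.
; When a Player actor overlaps it, it increments BearCount on player 0's Character_Blueprint and destroys itself.
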(event `self.ReceiveBeginPlay`
  (bind _iconimage (`self.IconImage`))
  (bind _iconimage_2 (`self.IconImage`))
  ;[1 1 1] Bounce
  (`KismetSystemLibrary.MoveComponentTo` _iconimage (+ (.location (`SceneComponent.GetRelativeTransform` _iconimage)) (0.0 0.0 70.0)) (struct) true true 0.7 :!label _label)
  (`KismetSystemLibrary.MoveComponentTo` _iconimage_2 (+ (.location (`SceneComponent.GetRelativeTransform` _iconimage_2)) (0.0 0.0 -70.0)) (struct) true true 0.7)
  (goto _label))

(event `self.ReceiveActorBeginOverlap`
  (params (OtherActor :type "Actor Object Reference"))
  ;[1 1 1] Player Collision to pick up spirit charge
  (cast `/Game/Animals/Player/Player` OtherActor)
  (bind _ascharacter_blueprint (cast `/Game/Blueprints/Character_Blueprint` (`GameplayStatics.GetPlayerCharacter` 0)))
  (bind _result (`/Engine/EditorBlueprintResources/StandardMacros.IncrementInt` (`/Game/Blueprints/Character_Blueprint.BearCount` _ascharacter_blueprint))
    (:`  `
      (set `/Game/Blueprints/Character_Blueprint.BearCount` _result _ascharacter_blueprint)
      (`self.K2_DestroyActor`))))

(fn `UserConstructionScript`)
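; Lever actor that raises or lowers the linked LeverThing actors when the Player overlaps it.
; BeginPlay drops the targets 1000 units if DoesMoveUp is set, then endlessly bobs IconImage with chained MoveComponentTo calls.
; Overlap restarts one of two timelines by DoesMoveUp, writing absolute world Z.
; The timeline is started inside the ForEach loop, so its updates reach only the last array element.
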(event `self.ReceiveBeginPlay`
  (bind _iconimage (`self.IconImage`))
  (bind _iconimage_2 (`self.IconImage`))
  ;[1 1 1] Bounce
  (if (`self.doesMoveUp`)
    (for _array_element (`self.LeverThing`)
      (`self.K2_SetActorTransform` _array_element (`KismetMathLibrary.MakeTransform` (+ (.location (`self.GetTransform` _array_element)) (0.0 0.0 -1000.0)) (.rotation (`self.GetTransform` _array_element)) (.scale (`self.GetTransform` _array_element))) false false)))
  (`KismetSystemLibrary.MoveComponentTo` _iconimage (+ (.location (`SceneComponent.GetRelativeTransform` _iconimage)) (0.0 0.0 70.0)) (struct) true true 0.7 :!label _label)
  (`KismetSystemLibrary.MoveComponentTo` _iconimage_2 (+ (.location (`SceneComponent.GetRelativeTransform` _iconimage_2)) (0.0 0.0 -70.0)) (struct) true true 0.7)
  (goto _label))

(event `self.ReceiveActorBeginOverlap`
  (params (OtherActor :type "Actor Object Reference"))
  ;[1 1 1] Player Collision to pick up spirit charge
  (cast `/Game/Animals/Player/Player` OtherActor)
  (if (`self.doesMoveUp`)
    (for _array_element (`self.LeverThing`)
      (bind (_direction _newtrack_0) (`Timeline|Timeline_1` :!via `PlayFromStart`)
        (:`Update`
          (`self.K2_SetActorLocation` _array_element (`KismetMathLibrary.MakeVector` (.x (`self.K2_GetActorLocation` _array_element)) (.y (`self.K2_GetActorLocation` _array_element)) _newtrack_0) false false))))
    (else
      (for _array_element_2 (`self.LeverThing`)
        (bind (_direction_2 _newtrack_0_2) (`Timeline|Timeline_0` :!via `PlayFromStart`)
          (:`Update`
            (`self.K2_SetActorLocation` _array_element_2 (`KismetMathLibrary.MakeVector` (.x (`self.K2_GetActorLocation` _array_element_2)) (.y (`self.K2_GetActorLocation` _array_element_2)) _newtrack_0_2) false false)))))))

(fn `UserConstructionScript`)
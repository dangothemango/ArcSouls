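; Main menu camera actor that shows the intro screen and keeps its camera slowly drifting.
; On BeginPlay it adds the IntroScreen widget to the viewport, then chains latent MoveComponentTo calls in an endless loop.
; Each move offsets the camera from its current relative location, so the sideways sway cancels out over a cycle while the height climbs with every loop.
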(event `self.ReceiveBeginPlay`
  (bind _cameracomponent (`self.CameraComponent`))
  (bind _cameracomponent_2 (`self.CameraComponent`))
  (bind _cameracomponent_3 (`self.CameraComponent`))
  (bind _cameracomponent_4 (`self.CameraComponent`))
  (bind _returnvalue (`|CreateWidget` "/Game/Levels/IntroScreen.IntroScreen_C"))
  (`UserWidget.AddToViewport` _returnvalue 0)
  (`KismetSystemLibrary.MoveComponentTo` _cameracomponent (+ (.location (`SceneComponent.GetRelativeTransform` _cameracomponent)) (0.0 -20.0 30.0)) (struct) false false 5.0 :!label _label)
  (`KismetSystemLibrary.MoveComponentTo` _cameracomponent_3 (+ (.location (`SceneComponent.GetRelativeTransform` _cameracomponent_3)) (0.0 -40.0 -15.0)) (struct) false false 5.0)
  (`KismetSystemLibrary.MoveComponentTo` _cameracomponent_2 (+ (.location (`SceneComponent.GetRelativeTransform` _cameracomponent_2)) (0.0 20.0 30.0)) (struct) false false 5.0)
  (`KismetSystemLibrary.MoveComponentTo` _cameracomponent_4 (+ (.location (`SceneComponent.GetRelativeTransform` _cameracomponent_4)) (0.0 40.0 15.0)) (struct) false false 5.0)
  (goto _label))

(fn `UserConstructionScript`)
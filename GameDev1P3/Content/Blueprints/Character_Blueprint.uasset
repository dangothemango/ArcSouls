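; Character Blueprint providing an orbit-style camera rig with drag-to-look controls and smooth repositioning.
; Holding the MoveCamera input lets the horizontal and vertical axes drive controller yaw and inverted pitch.
; Custom events use two-second eased MoveComponentTo calls: MoveCamera sends the capsule to a preset Location, and AdjustCameraDistance moves the camera component.
; AdjustCameraDistance multiplies CameraDistance by zero, so the camera always targets its relative origin.
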(event `InputAction|MoveCamera`
  (params (Key :type "Key Structure" :default "AnyKey"))
  ;[1 1 1] Basic controls to rotate the camera
  (:`Pressed`
    (set `self.ButtonDown` true))
  (:`Released`
    (set `self.ButtonDown` false)))

(event `InputAxis|Horizontal`
  (params (AxisValue :type "Float (single-precision)"))
  ;[1 1 1] Basic controls to rotate the camera
  (if (`self.ButtonDown`)
    (`self.AddControllerYawInput` AxisValue)))

(event `self.ReceiveBeginPlay`)

(event `InputAxis|Verticle`
  (params (AxisValue :type "Float (single-precision)"))
  ;[1 1 1] Basic controls to rotate the camera
  (if (`self.ButtonDown`)
    (`self.AddControllerPitchInput` (* AxisValue -1.0))))

(event `self.ReceiveTick`
  (params (DeltaSeconds :type "Float (single-precision)")))

(event `AdjustCameraDistance`
  ;[1 1 1] Sets the camera distance to "Camera Distance". Note that the "CameraDistance" variable must be set first
  (`KismetSystemLibrary.MoveComponentTo` (`self.GetComponentByClass` "/Script/Engine.CameraComponent") (`KismetMathLibrary.MakeVector` (* (`self.Camera Distance`) 0.0)) (struct) true true 2.0))

(event `MoveCamera`
  ;[1 1 1] Move Camera to "Location" Set variable before calling MoveCamera.
  (`KismetSystemLibrary.MoveComponentTo` (`self.GetComponentByClass` "/Script/Engine.CapsuleComponent") (`self.Location`) (struct) true true 2.0))

(fn `UserConstructionScript`)